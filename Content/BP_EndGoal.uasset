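; BP_EndGoal is an end-goal actor that can slide itself to a fixed world position.
; It enables player 0's input on BeginPlay, and a Z debug key press starts the WinDance timeline when the Move flag is set.
; Each timeline update lerps the root from its current location toward the hardcoded point, so the motion compounds rather than following the curve directly.
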(event EventBeginPlay
  (Input|EnableInput (Game|GetPlayerController 0)))

(event Collision|EventActorBeginOverlap
  (params (OtherActor :type Actor%20Object%20Reference)))

(event EventTick
  (params (DeltaSeconds :type Float%20%28single-precision%29)))

(event Input|KeyboardEvents|DebugKeyZ
  (params (Key :type Key%20Structure :default "None") (ActionValue :type Input%20Action%20Value%20Structure))
  (:Pressed
    (if (Variables|Default|GetMove?)
      (if true
        (bind _newtrack_1 (Timeline|WinDance Play)
          (:Update
            (Transformation|SetWorldLocation (Variables|Default|GetDefaultSceneRoot) (Math|Vector|Lerp(Vector) (Transformation|GetWorldLocation (Variables|Default|GetDefaultSceneRoot)) "850.000000,400.000000,500.000000" _newtrack_1) false false)))))))

(fn ConstructionScript)